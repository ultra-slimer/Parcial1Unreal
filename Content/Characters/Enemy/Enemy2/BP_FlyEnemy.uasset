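; Flying enemy character that sets itself up from data and reports sight of the player to its AI.
; On BeginPlay, its Class enum selects a DT_Enemy row that supplies the skeletal mesh and max walk speed.
; Perception updates check the player pawn's first stimulus, set PlayerOnSight with debug prints, and write SeeingPlayer and Target to the blackboard.
; Target is always the player pawn, even when unseen.
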(event `self.ReceiveBeginPlay`
  (bind _returnvalue (`|GetDataTableRow` "/Game/Characters/Enemy/DT_Enemy.DT_Enemy" (`KismetStringLibrary.Conv_StringToName` (`|GetEnumeratorNameAsString` (`self.Class`))))
    (:`then`
      (bind (_mesh _speed) (break `/Game/Characters/Enemy/EnemyStructure` _returnvalue))
      (set `CharacterMovementComponent.MaxWalkSpeed` _speed (`self.CharacterMovement`))
      (`SkinnedMeshComponent.SetSkinnedAssetAndUpdate` (`self.Mesh`) _mesh true))))

(event `self.AIPerception.OnTargetPerceptionUpdated`
  (params (Actor :type "Actor Object Reference") (Stimulus :type "AIStimulus Structure"))
  (bind _info (`AIPerceptionComponent.GetActorsPerception` (`self.AIPerception`) (`GameplayStatics.GetPlayerPawn` 0)))
  (if (`.bSuccessfullySensed` (break `AIStimulus` (`|GetArrayItem` (`.LastSensedStimuli` (break `ActorPerceptionBlueprintInfo` _info)))))
    (`KismetSystemLibrary.PrintString` "Visible")
    (set `self.PlayerOnSight` true)
    (else
      (`KismetSystemLibrary.PrintString` "Not Visible")
      (set `self.PlayerOnSight` false)))
  (`BlackboardComponent.SetValueAsBool` (`AIBlueprintHelperLibrary.GetBlackboard` null) "SeeingPlayer" (`self.PlayerOnSight`))
  (`BlackboardComponent.SetValueAsObject` (`AIBlueprintHelperLibrary.GetBlackboard` null) "Target" (`GameplayStatics.GetPlayerPawn` 0)))

(fn `UserConstructionScript`)