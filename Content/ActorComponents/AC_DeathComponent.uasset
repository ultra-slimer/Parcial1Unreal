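; AC_DeathComponent is an actor component that handles the death of the actor it is attached to.
; It caches its owner on BeginPlay, and its Die event looks up the owner's AC_HealthComponent.
; If that component is valid and CurrentHealth is strictly below zero, it calls Drop on the owner's AC_InventoryComponent, without a validity check, then destroys the owner.
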(event `self.ReceiveBeginPlay`
  (set `self.Owner` (`self.GetOwner`)))

(event `Die`
  (bind _returnvalue (`Actor.GetComponentByClass` (`self.Owner`) "/Game/ActorComponents/AC_HealthComponent.AC_HealthComponent_C"))
  (`/Engine/EditorBlueprintResources/StandardMacros.IsValid` _returnvalue
    (:`Is Valid`
      (if (< (`/Game/ActorComponents/AC_HealthComponent.CurrentHealth` _returnvalue) 0.0)
        (`/Game/ActorComponents/AC_InventoryComponent.Drop` (`Actor.GetComponentByClass` (`self.Owner`) "/Game/ActorComponents/AC_InventoryComponent.AC_InventoryComponent_C"))
        (`Actor.K2_DestroyActor` (`self.Owner`))))))