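; AC_HealthComponent is an actor component that tracks its owner's health.
; TakeDamage subtracts the damage from CurrentHealth and broadcasts OnHealthChanged with max and current values.
; It then calls Die on the owner's AC_DeathComponent after every hit, with no health check.
; A zero-health check that would fire OnDead is present but disconnected, so it never runs.
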(event `self.ReceiveBeginPlay`
  (set `self.Owner` (`self.GetOwner`)))

(event `TakeDamage`
  (params (damage :type "Float (double-precision)"))
  (set `self.CurrentHealth` (- (`self.CurrentHealth`) damage))
  (`self.OnHealthChanged` (`self.MaxHealth`) (`self.CurrentHealth`))
  (`/Game/ActorComponents/AC_DeathComponent.Die` (`Actor.GetComponentByClass` (`self.Owner`) "/Game/ActorComponents/AC_DeathComponent.AC_DeathComponent_C")))