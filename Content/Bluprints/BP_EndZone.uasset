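; BP_EndZone is a level goal actor that shows the victory screen when the player reaches it.
; Its Cube starts with visibility toggled and collision off until EnableEndZone makes it visible and collidable.
; Cube overlap and hit share one path, which checks that the other actor's instigator is BP_ThirdPersonCharacter, then disables collision.
; It then finds BP_MainHUD, removes the main UI and calls ShowScreen on the victory UI.
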(event `self.ReceiveBeginPlay`
  (bind _cube (`self.Cube`))
  (`SceneComponent.ToggleVisibility` _cube false)
  (`PrimitiveComponent.SetCollisionEnabled` _cube "NoCollision"))

(event `self.Cube.OnComponentBeginOverlap`
  (params (OverlappedComponent :type "PrimitiveComponent Object Reference") (OtherActor :type "Actor Object Reference") (OtherComp :type "PrimitiveComponent Object Reference") (OtherBodyIndex :type Integer) (bFromSweep :type Boolean) (SweepResult :type "HitResult Structure (by ref)"))
  (`KismetSystemLibrary.PrintString` "Hit EndZone" true true (struct :`G` 1.0 :`B` 0.065018 :`A` 1.0) :!label _label)
  (cast `/Game/ThirdPerson/Blueprints/BP_ThirdPersonCharacter` (`self.GetInstigator` (stale `self.Cube.OnComponentHit` OtherActor)))
  (`KismetSystemLibrary.PrintString` "EndZone Collided wit Player")
  (`PrimitiveComponent.SetCollisionEnabled` (`self.Cube`) "NoCollision")
  (bind _returnvalue (`GameplayStatics.GetActorOfClass` "/Game/FrameWork/UI/BP_MainHUD.BP_MainHUD_C"))
  (`Widget.RemoveFromParent` (`/Game/FrameWork/UI/BP_MainHUD.MainUI_Ref` _returnvalue))
  (`/Game/Blueprints/WBP_Victory.ShowScreen` (`/Game/FrameWork/UI/BP_MainHUD.VictoryUI_Ref` _returnvalue)))

(event `self.Cube.OnComponentHit`
  (params (HitComponent :type "PrimitiveComponent Object Reference") (OtherActor :type "Actor Object Reference") (OtherComp :type "PrimitiveComponent Object Reference") (NormalImpulse :type "Vector Structure") (Hit :type "HitResult Structure (by ref)"))
  (goto _label))

(fn `EnableEndZone`
  (bind _cube (`self.Cube`))
  (`SceneComponent.SetVisibility` _cube true true)
  (`PrimitiveComponent.SetCollisionEnabled` _cube "QueryAndPhysics")
  (`KismetSystemLibrary.PrintString` "Enabled EndZone" true true (struct :`R` 1.0 :`G` 0.054088 :`A` 1.0))
  (return))

(fn `UserConstructionScript`)