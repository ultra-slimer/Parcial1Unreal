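; BP_Collectable is a spinning coin pickup that the third-person player collects by overlapping it.
; Tick rotates the mesh by RotationSpeed each frame, without delta-time scaling.
; On overlap, it casts the other actor's instigator to BP_ThirdPersonCharacter, increments its Coins, updates the HUD and destroys itself.
; When it is the last collectable in the level, it enables the BP_EndZone before being destroyed.
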(event `self.ReceiveBeginPlay`)

(event `self.ReceiveTick`
  (params (DeltaSeconds :type "Float (single-precision)"))
  (`SceneComponent.K2_AddRelativeRotation` (`self.Mesh`) (`KismetMathLibrary.MakeRotator` 0.0 0.0 (`self.RotationSpeed`)) false false))

(event `self.Collider.OnComponentBeginOverlap`
  (params (OverlappedComponent :type "PrimitiveComponent Object Reference") (OtherActor :type "Actor Object Reference") (OtherComp :type "PrimitiveComponent Object Reference") (OtherBodyIndex :type Integer) (bFromSweep :type Boolean) (SweepResult :type "HitResult Structure (by ref)"))
  (bind _asbp_third_person_character (cast `/Game/ThirdPerson/Blueprints/BP_ThirdPersonCharacter` (`self.GetInstigator` OtherActor)))
  (`/Engine/EditorBlueprintResources/StandardMacros.IsValid` (`self.HUD`)
    (:`Is Valid`
      _)
    (:`Is Not Valid`
      (set `self.HUD` (`/Game/ThirdPerson/Blueprints/BP_ThirdPersonCharacter.HUD` _asbp_third_person_character))))
  (bind _result (`/Engine/EditorBlueprintResources/StandardMacros.IncrementInt` (`/Game/ThirdPerson/Blueprints/BP_ThirdPersonCharacter.Coins` _asbp_third_person_character))
    (:`  `
      (`KismetSystemLibrary.PrintString` (`KismetStringLibrary.Conv_IntToString` _result))
      (`/Game/Widgets/WBP_MainUI.ModifyCoin` (`self.HUD`) _result)
      (bind _outactors (`GameplayStatics.GetAllActorsOfClass` "BP_Collectable_C"))
      (bind _returnvalue (`KismetArrayLibrary.Array_Length` _outactors))
      (`KismetSystemLibrary.PrintString` (`KismetStringLibrary.Concat_StrStr` "Remaining Coins" (`KismetStringLibrary.Conv_IntToString` _returnvalue)))
      (if (<= _returnvalue 1)
        (bind _returnvalue_2 (`GameplayStatics.GetActorOfClass` "/Game/Bluprints/BP_EndZone.BP_EndZone_C"))
        (`/Game/Bluprints/BP_EndZone.EnableEndZone` _returnvalue_2))
      (`self.K2_DestroyActor`))))

(fn `UserConstructionScript`)